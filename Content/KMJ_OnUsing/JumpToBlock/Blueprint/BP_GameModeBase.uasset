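; Game mode for the JumpToBlock game that scores the player by elapsed play time.
; BeginPlay creates the score UI and adds it to the viewport, while GameStart and GameEnd toggle the gaming flag.
; While gaming, Tick accumulates time and passes whole seconds to AddScore, which overwrites the current score rather than adding to it.
; AddScore does nothing when its boolean parameter is true.
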(event Custom|GameStart
  (Variables|Default|SetIsGaming true))

(event Custom|GameEnd
  (Variables|Default|SetIsGaming false))

(event EventBeginPlay
  (bind _returnvalue (UserInterface|CreateWidget "/Game/KMJ_OnUsing/JumpToBlock/WidgetBP/ScoreUI.ScoreUI_C"))
  (UserInterface|Viewport|AddtoViewport _returnvalue 0))

(event EventTick
  (params (DeltaSeconds :type Float%20%28single-precision%29))
  (if (Variables|Default|GetIsGaming)
    (bind _output_get (Variables|Default|SetTimePass (+ (Variables|Default|GetTimePass) DeltaSeconds)))
    (CallFunction|AddScore (Math|Float|Truncate _output_get) false)))

(fn ConstructionScript)

(fn AddScore
  (params (Point :type Integer) (NewParam :type Boolean))
  (if (not NewParam)
    (Variables|Default|SetCurrentScore Point)))